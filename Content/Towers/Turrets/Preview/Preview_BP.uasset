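; Turret placement preview actor that shows whether its current location is a valid build spot.
; Each tick, capsule overlap tests require a TriggerBox as buildable area and reject spots overlapping enemies or other turrets.
; The result sets GoodBuildLocation on the Player_PlayerController and tints the Cylinder green or red through a dynamic material instance, which is requested every tick.
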(event EventTick
  (params (DeltaSeconds :type Float%20%28single-precision%29))
  ;[1 1 1] Tick
  (bind _asplayer_player_controller (Utilities|Casting|CastToPlayer_PlayerController (Game|GetPlayerController 0)))
  ;;[1 1 1] Check That Preview Is In  Buildable Area
  (bind _returnvalue (Collision|CapsuleOverlapActors (Transformation|GetActorLocation self) 1e+02 0.0 (Utilities|Array|MakeArray "ObjectTypeQuery2") "/Script/Engine.TriggerBox"))
  (if _returnvalue
    ;;[1 1 1] Check For Overlap With Enemys Or Other Turrets
    (bind _returnvalue_2 (Collision|CapsuleOverlapActors (Transformation|GetActorLocation self) 1e+02 0.0 (Utilities|Array|MakeArray "ObjectTypeQuery3") "/Game/BasicTowerDefense/Demo/Enemy_Master_BP.Enemy_Master_BP_C"))
    (if _returnvalue_2
      ;;[1 1 1] Set Ok To Build Variable
      (Variables|/Game/BasicTowerDefense/Player/Player_PlayerController.Player_PlayerController_C|SetGoodBuildLocation _asplayer_player_controller false :!label _label)
      ;;[1 1 1] Set The Preview Color
      (Variables|Default|Setcolor "(R=0.739583,G=0.000000,B=0.006992,A=1.000000)")
      (else
        (bind _returnvalue_3 (Collision|CapsuleOverlapActors (Transformation|GetActorLocation self) 1e+02 0.0 (Utilities|Array|MakeArray "ObjectTypeQuery3") "/Game/BasicTowerDefense/Turrets/Turret_Master_BP.Turret_Master_BP_C"))
        (if _returnvalue_3
          (goto _label)
          (else
            (Variables|/Game/BasicTowerDefense/Player/Player_PlayerController.Player_PlayerController_C|SetGoodBuildLocation _asplayer_player_controller true)
            (Variables|Default|Setcolor "(R=0.039926,G=0.286458,B=0.073283,A=1.000000)")))))
    (else
      (goto _label)))
  (bind _returnvalue_4 (Rendering|Material|CreateDynamicMaterialInstance (Variables|Default|GetCylinder) 0 0 "None" :!class /Script/Engine.PrimitiveComponent))
  (Rendering|Material|SetVectorParameterValue _returnvalue_4 "color" (Variables|Default|Getcolor) :!class /Script/Engine.MaterialInstanceDynamic))

(fn ConstructionScript)